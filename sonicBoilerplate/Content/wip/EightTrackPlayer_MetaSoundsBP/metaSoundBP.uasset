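; Eight-track stem player Blueprint that starts multitrack audio playback when play begins.
; BeginPlay spawns the Stem sound in 2D, then a Sequence passes eight track assets and their gains to it as named wave and float parameters.
; The asset and folder names indicate Stem is a MetaSound, with track selection and levels set by Blueprint variables once at startup.
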(event EventBeginPlay
  (bind _returnvalue (Audio|SpawnSound2D "/Game/BoilerAudio/Metasounds/stem.stem" 1.0 1.0 0.0 0))
  (Utilities|FlowControl|Sequence
    (:then_0
      ;[1 1 1] AudioSelection
      (Audio|Parameter|SetObjectParameter _returnvalue "Wave Asset 0" (Variables|Default|GetTrack0))
      ;[1 1 1] Gain
      (Audio|Parameter|SetFloatParameter _returnvalue "Gain 0" (Variables|Default|GetGain0) :!class /Script/AudioExtensions.AudioParameterControllerInterface))
    (:then_1
      (Audio|Parameter|SetObjectParameter _returnvalue "Wave Asset 1" (Variables|Default|GetTrack1))
      (Audio|Parameter|SetFloatParameter _returnvalue "Gain 1" (Variables|Default|GetGain%201) :!class /Script/AudioExtensions.AudioParameterControllerInterface))
    (:then_2
      (Audio|Parameter|SetObjectParameter _returnvalue "Wave Asset 2" (Variables|Default|GetTrack2))
      (Audio|Parameter|SetFloatParameter _returnvalue "Gain 2" (Variables|Default|GetGain%202) :!class /Script/AudioExtensions.AudioParameterControllerInterface))
    (:then_3
      (Audio|Parameter|SetObjectParameter _returnvalue "Wave Asset 3" (Variables|Default|GetTrack3))
      (Audio|Parameter|SetFloatParameter _returnvalue "Gain 3" (Variables|Default|GetGain%203) :!class /Script/AudioExtensions.AudioParameterControllerInterface))
    (:then_4
      (Audio|Parameter|SetObjectParameter _returnvalue "Wave Asset 4" (Variables|Default|GetTrack%204))
      (Audio|Parameter|SetFloatParameter _returnvalue "Gain 4" (Variables|Default|GetGain%204) :!class /Script/AudioExtensions.AudioParameterControllerInterface))
    (:then_5
      (Audio|Parameter|SetObjectParameter _returnvalue "Wave Asset 5" (Variables|Default|GetTrack%205))
      (Audio|Parameter|SetFloatParameter _returnvalue "Gain 5" (Variables|Default|GetGain%205) :!class /Script/AudioExtensions.AudioParameterControllerInterface))
    (:then_6
      (Audio|Parameter|SetObjectParameter _returnvalue "Wave Asset 6" (Variables|Default|GetTrack6))
      (Audio|Parameter|SetFloatParameter _returnvalue "Gain 6" (Variables|Default|GetGain%206) :!class /Script/AudioExtensions.AudioParameterControllerInterface))
    (:then_7
      (Audio|Parameter|SetObjectParameter _returnvalue "Wave Asset 7" (Variables|Default|GetTrack7))
      (Audio|Parameter|SetFloatParameter _returnvalue "Gain 7" (Variables|Default|GetGain%207) :!class /Script/AudioExtensions.AudioParameterControllerInterface))))

(fn ConstructionScript)
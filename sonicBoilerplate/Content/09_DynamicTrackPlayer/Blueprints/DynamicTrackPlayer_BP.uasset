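; Actor that plays a dynamic music track with adjustable pitch shift and gain through its Audio component.
; On BeginPlay it creates the track player HUD widget, hands it a self reference, shows the mouse cursor and passes the Track wave to the audio graph.
; Tick pushes the PitchShift and Gain0 variables into the audio component's named float parameters every frame, so changes apply live.
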(event EventBeginPlay
  (Utilities|FlowControl|Sequence
    (:then_0
      (bind _returnvalue (UserInterface|CreateWidget "/Game/UI/DynamicTackPlayer_HUD.DynamicTackPlayer_HUD_C" (Game|GetPlayerController 0)))
      (Variables|/Game/UI/DynamicTackPlayer_HUD.DynamicTackPlayer_HUD_C|SetTrackPlayerBP _returnvalue self)
      (UserInterface|Viewport|AddtoViewport _returnvalue 0)
      (Variables|/Script/Engine.PlayerController|SetbShowMouseCursor (Game|GetPlayerController 0) true))
    (:then_1
      (Class|AudioComponent|SetWaveParameter (Variables|Default|GetAudio) "WaveAsset" (Variables|Default|GetTrack)))))

(event Collision|EventActorBeginOverlap
  (params (OtherActor :type Actor%20Object%20Reference)))

(event EventTick
  (params (DeltaSeconds :type Float%20%28single-precision%29))
  (bind _audio (Variables|Default|GetAudio))
  (Audio|Parameter|SetFloatParameter _audio "PitchShift" (Variables|Default|GetPitchShift) :!class /Script/Engine.AudioComponent)
  (Audio|Parameter|SetFloatParameter _audio "Gain0" (Variables|Default|GetGain0) :!class /Script/Engine.AudioComponent))

(fn ConstructionScript)
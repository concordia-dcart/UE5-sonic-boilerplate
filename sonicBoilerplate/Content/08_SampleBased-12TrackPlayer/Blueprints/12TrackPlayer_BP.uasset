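; Twelve-track sample player actor that feeds wave assets and mix settings into the TrackPlayerPatch audio component.
; On BeginPlay it creates the TackPlayer_HUD widget with a reference to itself, shows the mouse cursor and assigns the twelve track waves as named parameters.
; Tick pushes the shared PitchShift and each track's volume variable to the patch's float parameters every frame, with an initial push at the end of BeginPlay.
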(event EventBeginPlay
  (bind _trackplayerpatch (Variables|MS_Patch|GetTrackPlayerPatch))
  (bind _trackplayerpatch_2 (Variables|MS_Patch|GetTrackPlayerPatch))
  (Utilities|FlowControl|Sequence
    (:then_0
      (bind _returnvalue (UserInterface|CreateWidget "/Game/UI/TackPlayer_HUD.TackPlayer_HUD_C" (Game|GetPlayerController 0)))
      (Variables|/Game/UI/TackPlayer_HUD.TackPlayer_HUD_C|Set12TrackBP _returnvalue self)
      (UserInterface|Viewport|AddtoViewport _returnvalue 0)
      (Variables|/Script/Engine.PlayerController|SetbShowMouseCursor (Game|GetPlayerController 0) true))
    (:then_1
      (Class|AudioComponent|SetWaveParameter _trackplayerpatch "Track01" (Variables|MS_Tracks|GetTrack01))
      (Class|AudioComponent|SetWaveParameter _trackplayerpatch "Track02" (Variables|MS_Tracks|GetTrack02))
      (Class|AudioComponent|SetWaveParameter _trackplayerpatch "Track03" (Variables|MS_Tracks|GetTrack03))
      (Class|AudioComponent|SetWaveParameter _trackplayerpatch "Track04" (Variables|MS_Tracks|GetTrack04))
      (Class|AudioComponent|SetWaveParameter _trackplayerpatch "Track05" (Variables|MS_Tracks|GetTrack05))
      (Class|AudioComponent|SetWaveParameter _trackplayerpatch "Track06" (Variables|MS_Tracks|GetTrack06))
      (Class|AudioComponent|SetWaveParameter _trackplayerpatch "Track07" (Variables|MS_Tracks|GetTrack07))
      (Class|AudioComponent|SetWaveParameter _trackplayerpatch "Track08" (Variables|MS_Tracks|GetTrack08))
      (Class|AudioComponent|SetWaveParameter _trackplayerpatch "Track09" (Variables|MS_Tracks|GetTrack09))
      (Class|AudioComponent|SetWaveParameter _trackplayerpatch "Track10" (Variables|MS_Tracks|GetTrack10))
      (Class|AudioComponent|SetWaveParameter _trackplayerpatch "Track11" (Variables|MS_Tracks|GetTrack11))
      (Class|AudioComponent|SetWaveParameter _trackplayerpatch "Track12" (Variables|MS_Tracks|GetTrack12)))
    (:then_2
      (Audio|Parameter|SetFloatParameter _trackplayerpatch_2 "PitchShift" (Variables|MS_Tempo|GetPitchShift) :!class /Script/Engine.AudioComponent)
      (Audio|Parameter|SetFloatParameter _trackplayerpatch_2 "Gain1" (Variables|MS_Volume|GetVolume01) :!class /Script/Engine.AudioComponent)
      (Audio|Parameter|SetFloatParameter _trackplayerpatch_2 "Gain2" (Variables|MS_Volume|GetVolume02) :!class /Script/Engine.AudioComponent)
      (Audio|Parameter|SetFloatParameter _trackplayerpatch_2 "Gain3" (Variables|MS_Volume|GetVolume03) :!class /Script/Engine.AudioComponent)
      (Audio|Parameter|SetFloatParameter _trackplayerpatch_2 "Gain4" (Variables|MS_Volume|GetVolume04) :!class /Script/Engine.AudioComponent)
      (Audio|Parameter|SetFloatParameter _trackplayerpatch_2 "Gain5" (Variables|MS_Volume|GetVolume05) :!class /Script/Engine.AudioComponent)
      (Audio|Parameter|SetFloatParameter _trackplayerpatch_2 "Gain6" (Variables|MS_Volume|GetVolume06) :!class /Script/Engine.AudioComponent)
      (Audio|Parameter|SetFloatParameter _trackplayerpatch_2 "Gain7" (Variables|MS_Volume|GetVolume07) :!class /Script/Engine.AudioComponent)
      (Audio|Parameter|SetFloatParameter _trackplayerpatch_2 "Gain8" (Variables|MS_Volume|GetVolume08) :!class /Script/Engine.AudioComponent)
      (Audio|Parameter|SetFloatParameter _trackplayerpatch_2 "Gain9" (Variables|MS_Volume|GetVolume09) :!class /Script/Engine.AudioComponent)
      (Audio|Parameter|SetFloatParameter _trackplayerpatch_2 "Gain10" (Variables|MS_Volume|GetVolume10) :!class /Script/Engine.AudioComponent)
      (Audio|Parameter|SetFloatParameter _trackplayerpatch_2 "Gain11" (Variables|MS_Volume|GetVolume11) :!class /Script/Engine.AudioComponent)
      (Audio|Parameter|SetFloatParameter _trackplayerpatch_2 "Gain12" (Variables|MS_Volume|GetVolume12) :!class /Script/Engine.AudioComponent))))

(event Collision|EventActorBeginOverlap
  (params (OtherActor :type Actor%20Object%20Reference)))

(event EventTick
  (params (DeltaSeconds :type Float%20%28single-precision%29))
  (bind _trackplayerpatch (Variables|MS_Patch|GetTrackPlayerPatch))
  (Audio|Parameter|SetFloatParameter _trackplayerpatch "PitchShift" (Variables|MS_Tempo|GetPitchShift) :!class /Script/Engine.AudioComponent)
  (Audio|Parameter|SetFloatParameter _trackplayerpatch "Gain1" (Variables|MS_Volume|GetVolume01) :!class /Script/Engine.AudioComponent)
  (Audio|Parameter|SetFloatParameter _trackplayerpatch "Gain2" (Variables|MS_Volume|GetVolume02) :!class /Script/Engine.AudioComponent)
  (Audio|Parameter|SetFloatParameter _trackplayerpatch "Gain3" (Variables|MS_Volume|GetVolume03) :!class /Script/Engine.AudioComponent)
  (Audio|Parameter|SetFloatParameter _trackplayerpatch "Gain4" (Variables|MS_Volume|GetVolume04) :!class /Script/Engine.AudioComponent)
  (Audio|Parameter|SetFloatParameter _trackplayerpatch "Gain5" (Variables|MS_Volume|GetVolume05) :!class /Script/Engine.AudioComponent)
  (Audio|Parameter|SetFloatParameter _trackplayerpatch "Gain6" (Variables|MS_Volume|GetVolume06) :!class /Script/Engine.AudioComponent)
  (Audio|Parameter|SetFloatParameter _trackplayerpatch "Gain7" (Variables|MS_Volume|GetVolume07) :!class /Script/Engine.AudioComponent)
  (Audio|Parameter|SetFloatParameter _trackplayerpatch "Gain8" (Variables|MS_Volume|GetVolume08) :!class /Script/Engine.AudioComponent)
  (Audio|Parameter|SetFloatParameter _trackplayerpatch "Gain9" (Variables|MS_Volume|GetVolume09) :!class /Script/Engine.AudioComponent)
  (Audio|Parameter|SetFloatParameter _trackplayerpatch "Gain10" (Variables|MS_Volume|GetVolume10) :!class /Script/Engine.AudioComponent)
  (Audio|Parameter|SetFloatParameter _trackplayerpatch "Gain11" (Variables|MS_Volume|GetVolume11) :!class /Script/Engine.AudioComponent)
  (Audio|Parameter|SetFloatParameter _trackplayerpatch "Gain12" (Variables|MS_Volume|GetVolume12) :!class /Script/Engine.AudioComponent))

(fn ConstructionScript)